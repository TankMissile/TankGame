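; Player-controllable tank pawn Blueprint that turns input into aiming, driving and firing.
; BeginPlay passes the Barrel and Turret components to their reference setters.
; Aim axes rotate a yaw gimbal and pitch arm, scaled by delta time for frame-rate independence.
; Movement supports both direct per-tread throttle and forward intent through MovementComponent, while the Fire action calls Fire.
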(event `self.ReceiveBeginPlay`
  (`self.SetBarrelReference` (`self.Barrel`))
  (`self.SetTurretReference` (`self.Turret`)))

(event `InputAxis|AimAzimuth`
  (params (AxisValue :type "Float (single-precision)"))
  ;[1 1 1] Aim Input Setup
  (`SceneComponent.K2_AddLocalRotation` (`self.YawGimble`) (`KismetMathLibrary.MakeRotator` 0.0 0.0 (* AxisValue 100.0 (`GameplayStatics.GetWorldDeltaSeconds`))) false false))

(event `InputAxis|LeftTreadThrottle`
  (params (AxisValue :type "Float (single-precision)"))
  ;[1 1 1] Movement Input Setup
  (`TankTread.SetThrottle` (`self.Tread_L`) AxisValue))

(event `InputAxis|AimElevation`
  (params (AxisValue :type "Float (single-precision)"))
  ;[1 1 1] Aim Input Setup
  (`SceneComponent.K2_AddLocalRotation` (`self.PitchArm`) (`KismetMathLibrary.MakeRotator` 0.0 (* AxisValue 100.0 (`GameplayStatics.GetWorldDeltaSeconds`))) false false))

(event `InputAxis|RightTreadThrottle`
  (params (AxisValue :type "Float (single-precision)"))
  ;[1 1 1] Movement Input Setup
  (`TankTread.SetThrottle` (`self.Tread_R`) AxisValue))

(event `InputAction|Fire`
  (params (Key :type "Key Structure" :default "AnyKey"))
  ;[1 1 1] Aim Input Setup
  (:`Pressed`
    (`self.Fire`)))

(event `InputAxis|Forward`
  (params (AxisValue :type "Float (single-precision)"))
  ;[1 1 1] Movement Input Setup
  (`TankMovementComponent.IntendMoveForward` (`self.MovementComponent`) AxisValue))

(fn `UserConstructionScript`)